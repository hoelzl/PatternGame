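; SelectionTrigger_BP is a trigger actor that lets the player pick a character by walking into it.
; When the player pawn overlaps, it writes its HelpText to the SelectionHUD widget held by SelectionGameMode and enables input on itself; leaving clears the text and disables input.
; While input is enabled, pressing E or Space passes its Character to the game mode's SelectCharacter.
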(event EventActorBeginOverlap
  (params (OtherActor :type Actor%20Object%20Reference))
  ;[1 1 1] Handle Overlap
  (if (== OtherActor (Game|Player|GetPlayerPawn 0))
    (Variables|/Game/Blueprints/SelectionHUD.SelectionHUD_C|SetHelpText (.AsSelection%20HUD (Utilities|Casting|CastToSelectionHUD (Variables|/Script/PG.SelectionGameMode|GetHUDWidget (.AsSelection%20Game%20Mode (Utilities|Casting|CastToSelectionGameMode (Game|GetGameMode)))))) (Variables|Help|GetHelpText))
    (Input|EnableInput (Game|GetPlayerController 0))))

(event Collision|EventActorEndOverlap
  (params (OtherActor :type Actor%20Object%20Reference))
  ;[1 1 1] Handle Overlap
  (if (== OtherActor (Game|Player|GetPlayerPawn 0))
    (Variables|/Game/Blueprints/SelectionHUD.SelectionHUD_C|SetHelpText (.AsSelection%20HUD (Utilities|Casting|CastToSelectionHUD (Variables|/Script/PG.SelectionGameMode|GetHUDWidget (.AsSelection%20Game%20Mode (Utilities|Casting|CastToSelectionGameMode (Game|GetGameMode)))))) "")
    (Input|DisableInput (Game|GetPlayerController 0))))

(event Input|KeyboardEvents|SpaceBar
  (params (Key :type Key%20Structure :default "AnyKey"))
  ;[1 1 1] Character Selection
  (:Pressed
    (Class|SelectionGameMode|SelectCharacter (.AsSelection%20Game%20Mode (Utilities|Casting|CastToSelectionGameMode (Game|GetGameMode))) (Variables|CharacterSelection|GetCharacter))))

(event Input|KeyboardEvents|E
  (params (Key :type Key%20Structure :default "AnyKey"))
  ;[1 1 1] Character Selection
  (:Pressed
    (Class|SelectionGameMode|SelectCharacter (.AsSelection%20Game%20Mode (Utilities|Casting|CastToSelectionGameMode (Game|GetGameMode))) (Variables|CharacterSelection|GetCharacter))))

(fn ConstructionScript)